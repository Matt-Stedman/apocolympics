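; Floating panel Blueprint that eases its panel back toward its starting pose while no Character stands on it.
; BeginPlay stores the panel's world transform, and Tick checks StepOnCollision for overlapping Characters.
; When none overlap, MoveComponentTo eases over one second, using the panel's linear and angular damping as the fraction of offset to remove.
; The targets are computed in world space but passed as relative location and rotation.
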(event `self.ReceiveBeginPlay`
  (set `self.Initial World Transform` (`SceneComponent.K2_GetComponentToWorld` (`self.floating_panel`))))

(event `self.ReceiveTick`
  (params (DeltaSeconds :type "Float (single-precision)"))
  (bind (_initial_world_transform_location _initial_world_transform_rotation) (`KismetMathLibrary.BreakTransform` (`self.Initial World Transform`)))
  (bind _floating_panel (`self.floating_panel`))
  (bind (_returnvalue_location _returnvalue_rotation) (`KismetMathLibrary.BreakTransform` (`SceneComponent.K2_GetComponentToWorld` _floating_panel)))
  (if (== (`KismetArrayLibrary.Array_Length` (`PrimitiveComponent.GetOverlappingActors` (`self.step_on_collision`) "/Script/Engine.Character")) 0)
    (`KismetSystemLibrary.MoveComponentTo` _floating_panel (- _returnvalue_location (* (- _returnvalue_location _initial_world_transform_location) (`PrimitiveComponent.GetLinearDamping` _floating_panel))) (`KismetMathLibrary.NormalizedDeltaRotator` _returnvalue_rotation (* (`KismetMathLibrary.NormalizedDeltaRotator` _returnvalue_rotation _initial_world_transform_rotation) (`PrimitiveComponent.GetAngularDamping` _floating_panel))) true true 1.0)))

(fn `UserConstructionScript`)