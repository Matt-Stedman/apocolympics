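; Swinging pole world object that characters with a Swinging component can grab and shimmy along.
; Overlapping the collision capsule calls HitPole on that component if it is not already swinging.
; End cap overlaps disable CanShimmyLeft or CanShimmyRight for swinging actors, re-enabling it on exit.
; The construction script sizes the mesh and capsule and positions both end caps from PoleLength.
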(event `self.Collision_Cap.OnComponentBeginOverlap`
  (params (OverlappedComponent :type "PrimitiveComponent Object Reference") (OtherActor :type "Actor Object Reference") (OtherComp :type "PrimitiveComponent Object Reference") (OtherBodyIndex :type Integer) (bFromSweep :type Boolean) (SweepResult :type "HitResult Structure (by ref)"))
  (bind (_contains_ _list_of_components) (`/Game/Gamification/Component_Helpers.Actor contains component class` OtherActor "/Game/Characters/Components/Motion/Swinging.Swinging_C"))
  (if _contains_
    (bind _asswinging (cast `/Game/Characters/Components/Motion/Swinging` (`|GetArrayItem` _list_of_components)))
    (if (not (`/Game/Characters/Components/Motion/Swinging.Is Swinging?` _asswinging))
      (`/Game/Characters/Components/Motion/Swinging.Hit Pole` _asswinging self))))

(event `self.Left End Cap.OnComponentBeginOverlap`
  (params (OverlappedComponent :type "PrimitiveComponent Object Reference") (OtherActor :type "Actor Object Reference") (OtherComp :type "PrimitiveComponent Object Reference") (OtherBodyIndex :type Integer) (bFromSweep :type Boolean) (SweepResult :type "HitResult Structure (by ref)"))
  (bind _asswinging (`self.Get Valid Swinging Component` OtherActor)
    (:`Is Valid`
      (set `/Game/Characters/Components/Motion/Swinging.Can Shimmy Left?` false _asswinging))))

(event `self.Left End Cap.OnComponentEndOverlap`
  (params (OverlappedComponent :type "PrimitiveComponent Object Reference") (OtherActor :type "Actor Object Reference") (OtherComp :type "PrimitiveComponent Object Reference") (OtherBodyIndex :type Integer))
  (bind _asswinging (`self.Get Valid Swinging Component` OtherActor)
    (:`Is Valid`
      (set `/Game/Characters/Components/Motion/Swinging.Can Shimmy Left?` true _asswinging))))

(event `self.Right End Cap.OnComponentBeginOverlap`
  (params (OverlappedComponent :type "PrimitiveComponent Object Reference") (OtherActor :type "Actor Object Reference") (OtherComp :type "PrimitiveComponent Object Reference") (OtherBodyIndex :type Integer) (bFromSweep :type Boolean) (SweepResult :type "HitResult Structure (by ref)"))
  (bind _asswinging (`self.Get Valid Swinging Component` OtherActor)
    (:`Is Valid`
      (set `/Game/Characters/Components/Motion/Swinging.Can Shimmy Right?` false _asswinging))))

(event `self.Right End Cap.OnComponentEndOverlap`
  (params (OverlappedComponent :type "PrimitiveComponent Object Reference") (OtherActor :type "Actor Object Reference") (OtherComp :type "PrimitiveComponent Object Reference") (OtherBodyIndex :type Integer))
  (bind _asswinging (`self.Get Valid Swinging Component` OtherActor)
    (:`Is Valid`
      (set `/Game/Characters/Components/Motion/Swinging.Can Shimmy Right?` true _asswinging))))

(fn `UserConstructionScript`
  (bind _pole_length (`self.Pole Length`))
  (`SceneComponent.SetRelativeScale3D` (`self.Pole`) (`KismetMathLibrary.MakeVector` (/ _pole_length 100.0) 1.0 1.0))
  (`CapsuleComponent.SetCapsuleHalfHeight` (`self.Collision_Cap`) (* _pole_length 8.2) true)
  (`SceneComponent.K2_SetRelativeLocation` (`self.Right End Cap`) (`KismetMathLibrary.MakeVector` (* _pole_length -9.0)) false false)
  (`SceneComponent.K2_SetRelativeLocation` (`self.Left End Cap`) (`KismetMathLibrary.MakeVector` (* _pole_length 9.0)) false false))